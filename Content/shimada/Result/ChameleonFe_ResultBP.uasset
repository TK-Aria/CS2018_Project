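; Chameleon actor for the Result folder that attaches itself to the player once its capsule is hit and counts as a capture.
; The hit event sets a mount flag, disables capsule collision and increments the capture count on MyGameInstance.
; While mounted, Tick copies player 0's location, with a slight Y offset, and rotation each frame instead of using component attachment.
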(event `self.ReceiveTick`
  (params (DeltaSeconds :type "Float (single-precision)"))
  (bind _returnvalue (`GameplayStatics.GetPlayerCharacter` 0))
  (if (`self.MountFlg`)
    (`self.K2_SetActorLocationAndRotation` (+ (`self.K2_GetActorLocation` _returnvalue) (0.0 1.0 0.0)) (`self.K2_GetActorRotation` _returnvalue))))

(event `self.CapsuleComponent.OnComponentHit`
  (params (HitComponent :type "PrimitiveComponent Object Reference") (OtherActor :type "Actor Object Reference") (OtherComp :type "PrimitiveComponent Object Reference") (NormalImpulse :type "Vector Structure") (Hit :type "HitResult Structure (by ref)"))
  (set `self.MountFlg` true)
  (`PrimitiveComponent.SetCollisionEnabled` (`self.CapsuleComponent`) "NoCollision")
  (bind _asmy_game_instance (cast `/Game/shimada/Result/MyGameInstance` (`GameplayStatics.GetGameInstance`)))
  (`/Game/shimada/Result/MyGameInstance.AddCountCapture` _asmy_game_instance))

(fn `UserConstructionScript`)